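; BP_IA is an enemy AI that heads for the first BP_Crystal found and switches to chasing the player once damaged.
; Tick reissues AIMoveTo, except briefly after HitSystem sets Hit, and advances a frame-counted attack timer.
; Sphere overlaps set the player or crystal target, which the timer damages through its HealthSystem.
; Its own HealthSystem caps health, flags being attacked and destroys the actor at zero.
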(event `Die`
  (`self.K2_DestroyActor`))

(event `HealthSystem`
  (params (Damage :type "Float (double-precision)"))
  (bind _healthmax (`self.HealthMax`))
  (bind _returnvalue (- (`self.Health`) Damage))
  ;[1 0.1557 0.7044] HealthSystem
  (if (<= _returnvalue 0.0)
    (`self.Die`)
    (elif (>= _returnvalue _healthmax)
      (set `self.Health` _healthmax)
      (else
        (set `self.Health` _returnvalue)
        (set `self.BeAttack` true)))))

(event `Timer`
  (bind _target_actor (`self.Target_Actor`))
  (bind _damage (`self.Damage`))
  (bind _returnvalue (+ (`self.I`) 1))
  ;[1 0.2187 0] HitSystem
  (if (`self.CanHit`)
    (if (>= _returnvalue (`self.I_Max`))
      (set `self.I` 0)
      (bind _asbp_player (cast `/Game/Blueprint/BP_Player` _target_actor)
        (:`then`
          (`/Game/Blueprint/BP_Player.HealthSystem` _asbp_player _damage))
        (:`CastFailed`
          (bind _asbp_crystal (cast `/Game/Blueprint/BP_Crystal` _target_actor))
          (`/Game/Blueprint/BP_Crystal.HealthSystem` _asbp_crystal _damage)))
      (else
        (set `self.I` _returnvalue)))
    (else
      (set `self.I` 0))))

(event `self.Sphere.OnComponentBeginOverlap`
  (params (OverlappedComponent :type "PrimitiveComponent Object Reference") (OtherActor :type "Actor Object Reference") (OtherComp :type "PrimitiveComponent Object Reference") (OtherBodyIndex :type Integer) (bFromSweep :type Boolean) (SweepResult :type "HitResult Structure (by ref)"))
  ;[1 0 0.005931] Id Hit
  (bind _asbp_player (cast `/Game/Blueprint/BP_Player` OtherActor)
    (:`then`
      (set `self.CanHit` true)
      (set `self.Target_Actor` _asbp_player))
    (:`CastFailed`
      (bind _asbp_crystal (cast `/Game/Blueprint/BP_Crystal` OtherActor))
      (set `self.CanHit` true)
      (set `self.Target_Actor` _asbp_crystal))))

(event `self.Sphere.OnComponentEndOverlap`
  (params (OverlappedComponent :type "PrimitiveComponent Object Reference") (OtherActor :type "Actor Object Reference") (OtherComp :type "PrimitiveComponent Object Reference") (OtherBodyIndex :type Integer))
  ;[1 0 0.005931] Id Hit
  (cast `/Game/Blueprint/BP_Player` OtherActor
    (:`then`
      (set `self.CanHit` false)
      (set `self.Target_Actor` null))
    (:`CastFailed`
      (cast `/Game/Blueprint/BP_Crystal` OtherActor)
      (set `self.CanHit` false)
      (set `self.Target_Actor` null))))

(event `self.ReceiveBeginPlay`
  ;[0 0.3018 1] Creation Id
  (bind _asbp_player (cast `/Game/Blueprint/BP_Player` (`GameplayStatics.GetPlayerPawn` 0)))
  (set `self.Player` _asbp_player)
  (bind _outactors (`GameplayStatics.GetAllActorsOfClass` "/Game/Blueprint/BP_Crystal.BP_Crystal_C"))
  (set `self.Crystal` (`|GetArrayItem` _outactors))
  (set `self.Health` (`self.HealthMax`)))

(event `self.ReceiveTick`
  (params (DeltaSeconds :type "Float (single-precision)"))
  (`|ExecutionSequence`
    (:`then_0`
      (if (not (`self.Hit`))
        (if (`self.BeAttack`)
          (`|AIMoveTo` self (0.0 0.0 0.0) (`self.Player`) 0.0)
          (else
            (`|AIMoveTo` self (0.0 0.0 0.0) (`self.Crystal`) 0.0)))))
    (:`then_1`
      (`self.Timer`))))

(event `HitSystem`
  (set `self.Hit` true)
  (`KismetSystemLibrary.Delay` 0.2)
  (set `self.Hit` false))

(fn `UserConstructionScript`)