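; BP_Crystal is a destructible crystal actor with a simple health pool that starts full on BeginPlay.
; Its HealthSystem event subtracts incoming damage, caps the result at HealthMax, and calls Die to destroy the actor when health would reach zero or below.
; A debug message prints whenever the new health lands between zero and the maximum.
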(event `HealthSystem`
  (params (Damage :type "Float (double-precision)"))
  (bind _healthmax (`self.HealthMax`))
  (bind _returnvalue (- (`self.Health`) Damage))
  ;[1 0.1557 0.7044] HealthSystem
  (if (<= _returnvalue 0.0)
    (`self.Die`)
    (elif (>= _returnvalue _healthmax)
      (set `self.Health` _healthmax)
      (else
        (set `self.Health` _returnvalue)
        (`KismetSystemLibrary.PrintString` "hit Crystal ")))))

(event `self.ReceiveBeginPlay`
  (set `self.Health` (`self.HealthMax`)))

(event `Die`
  (`self.K2_DestroyActor`))

(fn `UserConstructionScript`)