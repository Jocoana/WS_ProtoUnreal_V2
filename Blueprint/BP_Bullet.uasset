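; BP_Bullet is a homing projectile actor that damages BP_IA characters on impact.
; Each tick it moves toward its Target at constant speed set by Force without sweeping, then destroys itself if Target is invalid.
; Sphere hits ignore BP_Player; on a BP_IA they call HealthSystem with fixed damage, print its health and destroy the bullet.
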(event `self.ReceiveTick`
  (params (DeltaSeconds :type "Float (single-precision)"))
  (`self.K2_SetActorLocation` (`KismetMathLibrary.VInterpTo_Constant` (`self.K2_GetActorLocation`) (`self.K2_GetActorLocation` (`self.Target`)) (`GameplayStatics.GetWorldDeltaSeconds`) (`self.Force`)))
  (if (not (`KismetSystemLibrary.IsValid` (`self.Target`)))
    (`self.K2_DestroyActor`)))

(event `self.Sphere.OnComponentHit`
  (params (HitComponent :type "PrimitiveComponent Object Reference") (OtherActor :type "Actor Object Reference") (OtherComp :type "PrimitiveComponent Object Reference") (NormalImpulse :type "Vector Structure") (Hit :type "HitResult Structure (by ref)"))
  (cast `/Game/Blueprint/BP_Player` OtherActor
    (:`CastFailed`
      (bind _asbp_ia (cast `/Game/Blueprint/BP_IA` OtherActor))
      (`/Game/Blueprint/BP_IA.HealthSystem` _asbp_ia 5.0)
      (`KismetSystemLibrary.PrintString` (`KismetStringLibrary.Conv_DoubleToString` (`/Game/Blueprint/BP_IA.Health` _asbp_ia)))
      (`self.K2_DestroyActor`))))

(fn `UserConstructionScript`)